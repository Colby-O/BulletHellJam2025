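; BP_Boss is a boss enemy Blueprint whose events swap skeletal mesh materials to show its damaged, open, closed and rest states.
; Damaged and rest events change material slot 0, while open and closed events change slot 2 and also set slot 0 to rest or disabled.
; The construction script assigns the Shooter and SkeletalMesh components to ShooterComp and Mesh variables, and BeginPlay does nothing.
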(event `self.ReceiveBeginPlay`)

(event `self.SetDamagedMaterial`
  (`PrimitiveComponent.SetMaterial` (`self.SkeletalMesh`) 0 (`self.DamagedMat`)))

(event `self.SetOpenMaterial`
  (bind _skeletalmesh (`self.SkeletalMesh`))
  (`PrimitiveComponent.SetMaterial` _skeletalmesh 2 (`self.OpenMat`))
  (`PrimitiveComponent.SetMaterial` _skeletalmesh 0 (`self.RestMat`)))

(event `self.SetClosedMaterial`
  (bind _skeletalmesh (`self.SkeletalMesh`))
  (`PrimitiveComponent.SetMaterial` _skeletalmesh 2 (`self.ClosedMat`))
  (`PrimitiveComponent.SetMaterial` _skeletalmesh 0 (`self.DisabledMat`)))

(event `self.SetRestMaterial`
  (`PrimitiveComponent.SetMaterial` (`self.SkeletalMesh`) 0 (`self.RestMat`)))

(fn `UserConstructionScript`
  (set `self.ShooterComp` (`self.Shooter`))
  (set `self.Mesh` (`self.SkeletalMesh`)))